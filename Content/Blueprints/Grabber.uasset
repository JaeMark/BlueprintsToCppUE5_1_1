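; Grabber scene component that lets its owner pick up, carry and release physics objects.
; Tick moves the physics handle target to the hold location and component rotation.
; Grab is written to enable physics on a sphere-traced body, hold it by center of mass and notify quest actors.
; The trace function returns false regardless of hits, and NotifyQuestActorOld is an uncalled pickup-trigger notifier.
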(event `self.ReceiveTick`
  (params (DeltaSeconds :type "Float (single-precision)"))
  (`PhysicsHandleComponent.SetTargetLocationAndRotation` (`self.GetPhysicsComponent`) (`self.GetHoldLocation`) (`self.K2_GetComponentRotation`)))

(fn `Grab`
  (bind (_hitactor _hitcomponent _returnvalue) (`self.TraceForPhysicsBodies`))
  (if _returnvalue
    (`PrimitiveComponent.SetSimulatePhysics` _hitcomponent true) ; Some actors may not yet.
    (`PhysicsHandleComponent.GrabComponentAtLocationWithRotation` :`self` (`self.GetPhysicsComponent`) :`Component` _hitcomponent :`Location` (`PrimitiveComponent.GetCenterOfMass` _hitcomponent "None"))
    (`self.NotifyQuestActor` _hitactor)))

(fn `NotifyQuestActorOld`
  (params (Actor :type "Actor Object Reference"))
  (bind _returnvalue (`Actor.GetComponentByClass` Actor "/Game/Quests/CompletionTriggers/BP_QuestTriggerPickup.BP_QuestTriggerPickup_C"))
  (`/Engine/EditorBlueprintResources/StandardMacros.IsValid` _returnvalue
    (:`Is Valid`
      (`/Game/Quests/CompletionTriggers/BP_QuestTriggerPickup.Pickup` _returnvalue))))

(fn `Release`
  (`PhysicsHandleComponent.ReleaseComponent` (`self.GetPhysicsComponent`)))

(fn `TraceForPhysicsBodies`
  (returns (HitActor :type "Actor Object Reference") (HitComponent :type "PrimitiveComponent Object Reference") (ReturnValue :type Boolean))
  (bind _outhit (`KismetSystemLibrary.SphereTraceSingleForObjects` (`self.K2_GetComponentLocation`) (`self.GetMaxGrabLocation`) (`self.GrabRadius`) (`|MakeArray` "ObjectTypeQuery4" :!type "EObjectTypeQuery Enum")))
  (return null null false))